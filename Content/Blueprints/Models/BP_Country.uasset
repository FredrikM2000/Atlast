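; BP_Country is a country actor that starts lowered, rises when discovered and glows when clicked.
; On BeginPlay it creates a dynamic material on the Land mesh and sets its Z below zero.
; ObjClick prints the display name and plays a timeline driving the Emissive parameter at an adjustable speed.
; LandDiscovered matches the passed name against the actor's display name, then animates its height with a timeline.
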(event Custom|LandDiscovered
  (params (LandNavn :type String))
  (bind _returnvalue (Transformation|GetActorLocation))
  (bind (_x _y) (Math|Vector|BreakVector _returnvalue))
  (if (Utilities|Enum|Equal(Enum) LandNavn (Utilities|GetDisplayName self))
    (bind _zrise (Timeline|RiseLand_Timeline PlayFromStart)
      (:Update
        (Transformation|SetActorLocation (Math|Vector|MakeVector _x _y _zrise) false false)))))

(event EventBeginPlay
  (bind _returnvalue (Transformation|GetActorLocation))
  (bind (_x _y) (Math|Vector|BreakVector _returnvalue))
  (bind _returnvalue_2 (Rendering|Material|CreateDynamicMaterialInstance (Variables|Default|GetLand) 0 0 "None" :!class /Script/Engine.PrimitiveComponent))
  (Variables|Default|SetDynamic%20Material _returnvalue_2)
  (Transformation|SetActorLocation (Math|Vector|MakeVector _x _y -5e+01) false false))

(event Collision|EventActorBeginOverlap
  (params (OtherActor :type Actor%20Object%20Reference)))

(event EventTick
  (params (DeltaSeconds :type Float%20%28single-precision%29)))

(event EventObjClick
  (Development|PrintString (Utilities|GetDisplayName self) true true "(R=0.000000,G=0.660000,B=1.000000,A=1.000000)" 1.0)
  (Components|Timeline|SetPlayRate (Variables|Default|GetClicked) (Variables|Default|GetClickAnimationSpeed))
  (bind _newtrack_0 (Timeline|Clicked PlayFromStart)
    (:Update
      (Rendering|Material|SetScalarParameterValue (Variables|Default|GetDynamic%20Material) "Emissive" _newtrack_0 :!class /Script/Engine.MaterialInstanceDynamic))))

(fn ConstructionScript)