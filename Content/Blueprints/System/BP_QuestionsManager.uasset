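; BP_QuestionsManager is a manager actor that sets up the map for Norway at level start.
; On BeginPlay it clears the InQuestions flag, caches the BP_Kartet map actor and calls HvisLand on it, then LandDiscovered on every BP_Country, passing "Norge".
; After a short delay it calls ShowMarkers on every BP_Landmark, using "Norway" rather than "Norge".
; Despite its name, it contains no question logic beyond resetting that flag.
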(event EventBeginPlay
  (Variables|Default|SetInQuestions false)
  (bind _returnvalue (Actor|GetActorOfClass "/Game/Blueprints/BP_Kartet.BP_Kartet_C"))
  (Variables|Default|SetKartet _returnvalue)
  (Utilities|FlowControl|Sequence
    (:then_0
      (Default|HvisLand (Variables|Default|GetKartet) "Norge")
      (bind _outactors (Actor|GetAllActorsOfClass "/Game/Blueprints/Models/BP_Country.BP_Country_C"))
      (for _array_element _outactors
        (Default|LandDiscovered _array_element "Norge")))
    (:then_1
      (Utilities|FlowControl|Delay 0.5)
      (bind _outactors_2 (Actor|GetAllActorsOfClass "/Game/Blueprints/BP_Landmark.BP_Landmark_C"))
      (for _array_element_2 _outactors_2
        (Default|ShowMarkers _array_element_2 "Norway")))))

(event Collision|EventActorBeginOverlap
  (params (OtherActor :type Actor%20Object%20Reference)))

(event EventTick
  (params (DeltaSeconds :type Float%20%28single-precision%29)))

(fn ConstructionScript)