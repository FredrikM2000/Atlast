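; BP_ProgressManager unlocks countries in a fixed order (Sweden, Denmark, Finland, Iceland) as the game mode's progress passes rising thresholds.
; CheckProgress reads CurrentProgress from BP_AtlastGameModeBase and tests chained unlock flags.
; Each unlock calls HvisLand on the BP_Kartet found at BeginPlay, LandDiscovered on every BP_Country, then, after a short delay, ShowMarkers on every BP_Landmark.
; Map and country calls use Scandinavian names, while landmark markers use English ones.
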(event Custom|Check%20Progress
  (Development|PrintString "Checking Progress")
  (if (not (Variables|Default|GetUnlockedAllCountries))
    (bind _asbp_atlast_game_mode_base (Utilities|Casting|CastToBP_AtlastGameModeBase (Game|GetGameMode)))
    (bind _returnvalue (Class|AtlastGameModeBase|CurrentProgress _asbp_atlast_game_mode_base))
    (if (Variables|Default|GetUnlockedSweden)
      (if (Variables|Default|GetUnlockedDenmark) :!label _label
        (if (Variables|Default|GetUnlockedFinland) :!label _label_2
          (if (not (Variables|Default|GetUnlockedAllCountries)) :!label _label_3
            (if (>= _returnvalue 0.018)
              (Default|HvisLand (Variables|Default|GetKartet) "Island")
              (bind _outactors (Actor|GetAllActorsOfClass "/Game/Blueprints/Models/BP_Country.BP_Country_C"))
              (for _array_element _outactors
                (Default|LandDiscovered _array_element "Island")
                (Variables|Default|SetUnlockedAllCountries true)
                (Utilities|FlowControl|Delay 0.5)
                (bind _outactors_2 (Actor|GetAllActorsOfClass "/Game/Blueprints/BP_Landmark.BP_Landmark_C"))
                (for _array_element_2 _outactors_2
                  (Default|ShowMarkers _array_element_2 "Iceland")))))
          (elif (>= _returnvalue 0.0125)
            (Default|HvisLand (Variables|Default|GetKartet) "Finland")
            (bind _outactors_3 (Actor|GetAllActorsOfClass "/Game/Blueprints/Models/BP_Country.BP_Country_C"))
            (for _array_element_3 _outactors_3
              (Default|LandDiscovered _array_element_3 "Finland")
              (Variables|Default|SetUnlockedFinland true)
              (Utilities|FlowControl|Delay 0.5)
              (bind _outactors_4 (Actor|GetAllActorsOfClass "/Game/Blueprints/BP_Landmark.BP_Landmark_C"))
              (for _array_element_4 _outactors_4
                (Default|ShowMarkers _array_element_4 "Finland")
                (goto _label_3)))))
        (elif (>= _returnvalue 0.0075)
          (Default|HvisLand (Variables|Default|GetKartet) "Danmark")
          (bind _outactors_5 (Actor|GetAllActorsOfClass "/Game/Blueprints/Models/BP_Country.BP_Country_C"))
          (for _array_element_5 _outactors_5
            (Default|LandDiscovered _array_element_5 "Danmark")
            (Variables|Default|SetUnlockedDenmark true)
            (Utilities|FlowControl|Delay 0.5)
            (bind _outactors_6 (Actor|GetAllActorsOfClass "/Game/Blueprints/BP_Landmark.BP_Landmark_C"))
            (for _array_element_6 _outactors_6
              (Default|ShowMarkers _array_element_6 "Denmark")
              (goto _label_2)))))
      (elif (>= _returnvalue 0.003)
        (Default|HvisLand (Variables|Default|GetKartet) "Sverige")
        (bind _outactors_7 (Actor|GetAllActorsOfClass "/Game/Blueprints/Models/BP_Country.BP_Country_C"))
        (for _array_element_7 _outactors_7
          (Default|LandDiscovered _array_element_7 "Sverige")
          (Variables|Default|SetUnlockedSweden true)
          (Utilities|FlowControl|Delay 0.5)
          (bind _outactors_8 (Actor|GetAllActorsOfClass "/Game/Blueprints/BP_Landmark.BP_Landmark_C"))
          (for _array_element_8 _outactors_8
            (Default|ShowMarkers _array_element_8 "Sweden")
            (goto _label)))))))

(event EventBeginPlay
  (bind _returnvalue (Actor|GetActorOfClass "/Game/Blueprints/BP_Kartet.BP_Kartet_C"))
  (Variables|Default|SetKartet _returnvalue))

(event Collision|EventActorBeginOverlap
  (params (OtherActor :type Actor%20Object%20Reference)))

(event EventTick
  (params (DeltaSeconds :type Float%20%28single-precision%29)))

(fn ConstructionScript)