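; Player pawn for a map game with countries, landmarks and questions, handling mouse input and adding menu and intro widgets on BeginPlay.
; A hold timer separates clicks from drags; clicks trace two channels to message hit objects unless questions are active, while drag movement is disconnected.
; Tick traces camera-to-character to message occluders for dithering.
; Right mouse fades an emissive material parameter; key 5 is a progress cheat.
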(event Custom|LeftMouseRelease
  (bind _returnvalue (Game|GetPlayerController 0))
  (bind (_locationx _locationy) (Game|Player|GetMousePosition _returnvalue))
  ;[1 1 1] TICK
  (Utilities|FlowControl|DoOnce false) ; enters at Reset
)

(event EventBeginPlay
  (bind _returnvalue (Game|GetPlayerController 0))
  ;[1 1 1] Begin play
  (bind _returnvalue_2 (UserInterface|CreateWidget "/Game/UI_UX/Widgets/WBP_MainMenu2.WBP_MainMenu2_C" _returnvalue))
  (UserInterface|Viewport|AddtoViewport _returnvalue_2 0)
  (Variables|/Script/Engine.PlayerController|SetbShowMouseCursor _returnvalue true)
  (bind _returnvalue_3 (Actor|GetActorOfClass "/Game/Testing/Sprite_Testing/BP_SpriteCharacter.BP_SpriteCharacter_C"))
  (Variables|Default|SetSpriteCharacter _returnvalue_3)
  (bind _returnvalue_4 (Actor|GetActorOfClass "/Game/Blueprints/BP_Kartet.BP_Kartet_C"))
  (Variables|Default|SetKartet _returnvalue_4)
  (bind _returnvalue_5 (UserInterface|CreateWidget "/Game/UI_UX/Widgets/WBP_Intro.WBP_Intro_C" _returnvalue))
  (UserInterface|Viewport|AddtoViewport _returnvalue_5 0))

(event Collision|EventActorBeginOverlap
  (params (OtherActor :type Actor%20Object%20Reference)))

(event EventTick
  (params (DeltaSeconds :type Float%20%28single-precision%29))
  (bind _returnvalue (Game|GetPlayerController 0))
  (bind (_locationx _locationy) (Game|Player|GetMousePosition _returnvalue))
  ;[1 1 1] TICK
  (Utilities|FlowControl|Sequence
    (:then_0
      (if (Variables|Default|GetbLeftClickTimer)
        (Variables|Default|SetMouseLEFTClickTimer (+ (Variables|Default|GetMouseLEFTClickTimer) DeltaSeconds))
        (if (> (Variables|Default|GetMouseLEFTClickTimer) (Variables|Default|GetMoveOrClickTimer))
          (Utilities|FlowControl|DoOnce false
            (:Completed
              (Variables|Default|SetbMove true)
              (Variables|MouseMovement|SetLast%20MouseLocation%20X _locationx)
              (Variables|MouseMovement|SetLast%20Mouse%20Location%20Y _locationy))))))
    (:then_1
      (if (Variables|Default|GetbMove)
        (CallFunction|MouseMovement)))
    (:then_2
      (CallFunction|DitherObject))))

(event EventObjClick
  ;[1 1 1] On Object Click
)

(event Input|ActionEvents|InputActionLeftClick
  (params (Key :type Key%20Structure :default "None"))
  ;[1 1 1] Left Mouse
  (:Pressed
    (Variables|Default|SetbLeftClickTimer true))
  (:Released
    (Variables|Default|SetbLeftClickTimer false)
    (Utilities|FlowControl|Sequence
      (:then_0
        (if (> (Variables|Default|GetMoveOrClickTimer) (Variables|Default|GetMouseLEFTClickTimer))
          (CallFunction|ClickonObject)))
      (:then_1
        (Variables|Default|SetMouseLEFTClickTimer 0.0)
        (Variables|Default|SetbMove false)
        (CallFunction|LeftMouseRelease)))))

(event Input|ActionEvents|InputActionMouseWheelUp
  (params (Key :type Key%20Structure :default "None"))
  ;[1 1 1] Mouse wheel
)

(event Input|ActionEvents|InputActionMouseWheelDown
  (params (Key :type Key%20Structure :default "None"))
  ;[1 1 1] Mouse wheel
)

(event Input|MouseEvents|RightMouseButton
  (params (Key :type Key%20Structure :default "None"))
  ;[1 1 1] Right Mouse
  (:Pressed
    (bind _newtrack_0 (Timeline|Timeline_0 Play)
      (:Update
        (Rendering|Material|SetScalarParameterValue "/Game/Materials/MaterialLocationParameter.MaterialLocationParameter" "Emissive" _newtrack_0 :!class /Script/Engine.KismetMaterialLibrary))))
  (:Released
    (Timeline|Timeline_0 Reverse)))

(event Input|KeyboardEvents|1
  (params (Key :type Key%20Structure :default "None"))
  ;[1 1 1] Juksekode for å få fram land
)

(event Input|KeyboardEvents|2
  (params (Key :type Key%20Structure :default "None"))
  ;[1 1 1] Juksekode for å få fram land
)

(event Input|KeyboardEvents|3
  (params (Key :type Key%20Structure :default "None"))
  ;[1 1 1] Juksekode for å få fram land
)

(event Input|KeyboardEvents|4
  (params (Key :type Key%20Structure :default "None")))

(event Input|KeyboardEvents|5
  (params (Key :type Key%20Structure :default "None"))
  (:Pressed
    (bind _asbp_atlast_game_mode_base (Utilities|Casting|CastToBP_AtlastGameModeBase (Game|GetGameMode)))
    (Class|AtlastGameModeBase|IncreaseProgress _asbp_atlast_game_mode_base 500)
    (bind _returnvalue (Actor|GetActorOfClass "/Game/Blueprints/System/BP_ProgressManager.BP_ProgressManager_C"))
    (Default|CheckProgress _returnvalue)))

(fn ConstructionScript)

(fn MouseMovement)

(fn ClickonObject
  (bind _returnvalue (Game|GetPlayerController 0))
  (bind _returnvalue_2 (Game|GetPlayerController 0))
  (bind (_worldlocation _worlddirection) (Game|Player|ConvertMouseLocationToWorldSpace _returnvalue))
  (bind (_worldlocation_2 _worlddirection_2) (Game|Player|ConvertMouseLocationToWorldSpace _returnvalue_2))
  (bind _returnvalue_3 (Actor|GetActorOfClass "/Game/Blueprints/System/BP_QuestionsManager.BP_QuestionsManager_C"))
  (if (not (Variables|/Game/Blueprints/System/BP_QuestionsManager.BP_QuestionsManager_C|GetInQuestions _returnvalue_3))
    (Utilities|FlowControl|Sequence
      (:then_0
        (bind (_outhit _returnvalue_4) (Collision|LineTraceByChannel (Transformation|GetWorldLocation (Variables|Default|GetCamera)) (+ _worldlocation (* _worlddirection 1e+03)) "TraceTypeQuery3" true 0 "None"))
        (if _returnvalue_4
          (Class|ObjectClick|ObjClick(Message) (.HitActor (Collision|BreakHitResult _outhit)))))
      (:then_1
        (bind (_outhit_2 _returnvalue_5) (Collision|LineTraceByChannel (Transformation|GetWorldLocation (Variables|Default|GetCamera)) (+ _worldlocation_2 (* _worlddirection_2 1e+03)) "TraceTypeQuery4" true 0 "None"))
        (if _returnvalue_5
          (Class|LandemerkeonClick|OnClickLandemerke(Message) (.HitActor (Collision|BreakHitResult _outhit_2))))))))

(fn DitherObject
  (bind (_outhit _returnvalue) (Collision|LineTraceByChannel (Transformation|GetWorldLocation (Variables|Default|GetCamera)) (+ (Transformation|GetActorLocation (Variables|Default|GetSpriteCharacter)) "0, 0,30.000000") "TraceTypeQuery1" false 0 "None"))
  (if _returnvalue
    (Class|ObjectDithering|ObjectDithering(Message) (.HitActor (Collision|BreakHitResult _outhit)))))

(fn NewFunction0)