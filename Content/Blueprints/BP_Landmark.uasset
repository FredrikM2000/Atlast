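; BP_Landmark is a landmark marker actor that opens a quiz when clicked.
; On BeginPlay it sets a default marker sprite and hides itself until Showmarkers reveals it.
; OnClickLandemerke replaces any existing question widget with a new WBP_QuestionBase, passing its internal name and itself to build the question pool.
; CompleteQuiz swaps in the landmark's own sprite by name, currently only for the opera, while ChangeLandMark sets any given sprite.
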(event Custom|ChangeLandMark
  (params (Sprite :type Paper%20Sprite%20Object%20Reference))
  (Rendering|Components|Sprite|SetSprite (Variables|Default|GetPaperSprite) Sprite))

(event Custom|Show%20markers
  (Rendering|SetActorHiddenInGame false))

(event Custom|CompleteQuiz
  (switch string (Utilities|String|ToString(Text) (Variables|Default|GetInternalName))
    (:NorOpera
      (Rendering|Components|Sprite|SetSprite (Variables|Default|GetPaperSprite) "/Game/Sprites/Landemerker/operaen_Sprite.operaen_Sprite"))))

(event EventBeginPlay
  (Rendering|Components|Sprite|SetSprite (Variables|Default|GetPaperSprite) "/Game/Sprites/Landemerker/LandemerkeMarker_Sprite1.LandemerkeMarker_Sprite1")
  (Rendering|SetActorHiddenInGame true))

(event Collision|EventActorBeginOverlap
  (params (OtherActor :type Actor%20Object%20Reference)))

(event EventTick
  (params (DeltaSeconds :type Float%20%28single-precision%29)))

(event EventOnClickLandemerke
  (bind _aswidget (Utilities|Casting|CastToWidget (stale _returnvalue))
    (:then
      (Widget|RemovefromParent _aswidget))
    (:CastFailed
      _))
  (bind _returnvalue (UserInterface|CreateWidget "/Game/UI_UX/Widgets/Question/WBP_QuestionBase.WBP_QuestionBase_C"))
  (Default|CreateQuestionPool _returnvalue (Variables|Default|GetInternalName) self)
  (UserInterface|Viewport|AddtoViewport _returnvalue 0))

(fn ConstructionScript)