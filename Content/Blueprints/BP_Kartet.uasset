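; BP_Kartet is a map actor that animates the reveal of a land, chosen by material parameter name.
; BeginPlay creates a dynamic material instance on the mesh and applies a configurable play rate to the VisningAvLand timeline.
; The HvisLand event waits briefly, then plays that timeline from the start, writing its alpha into the scalar parameter named by the caller.
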(event Custom|Hvis%20Land
  (params (NewParam :type Name))
  (Utilities|FlowControl|Delay 0.5)
  (bind _alpha (Timeline|Visning%20av%20land PlayFromStart)
    (:Update
      (Rendering|Material|SetScalarParameterValue (Variables|Default|GetDynamicMaterial) NewParam _alpha :!class /Script/Engine.MaterialInstanceDynamic))))

(event EventBeginPlay
  (bind _returnvalue (Rendering|Material|CreateDynamicMaterialInstance (Variables|Character|GetMesh) 0 0 "None" :!class /Script/Engine.PrimitiveComponent))
  (Variables|Default|SetDynamicMaterial _returnvalue)
  (Components|Timeline|SetPlayRate (Variables|Default|GetVisning%20av%20land) (Variables|Default|GetAnimationSpeed%20VisningAvLand)))

(event Collision|EventActorBeginOverlap
  (params (OtherActor :type Actor%20Object%20Reference)))

(event EventTick
  (params (DeltaSeconds :type Float%20%28single-precision%29)))

(fn ConstructionScript)