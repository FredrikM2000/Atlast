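; Test sprite character that plays a running Paper2D flipbook and keeps itself snapped to the ground.
; Each tick it writes its centred, inverted screen position, normalised by viewport size, to a material parameter collection.
; It also traces vertically and moves to the hit height, drawing debug lines for the surface normal, up vector and an angle-rotated normal.
; The timeline-driven local offset is unconnected.
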(event EventBeginPlay
  (Sprite|SetFlipbook (Variables|Default|GetPaperFlipbook) (Variables|Default|GetRun%20FB)))

(event Collision|EventActorBeginOverlap
  (params (OtherActor :type Actor%20Object%20Reference)))

(event EventTick
  (params (DeltaSeconds :type Float%20%28single-precision%29))
  (CallFunction|GetActorScreenPosition)
  (CallFunction|GroundOffset))

(fn ConstructionScript)

(fn GetActorScreenPosition
  (bind _returnvalue (Viewport|GetViewportSize))
  (bind _returnvalue_2 (Transformation|GetActorLocation))
  (bind _returnvalue_3 (Game|GetPlayerController 0))
  (bind (_x _y) (Math|Vector2D|BreakVector2D _returnvalue))
  (bind _returnvalue_4 (+ _returnvalue_2 "0, 0,60.000000"))
  (bind _screenposition (Class|GameplayStatics|ProjectWorldtoScreen _returnvalue_3 _returnvalue_4 true))
  (bind (_x_2 _y_2) (Math|Vector2D|BreakVector2D _screenposition))
  (Rendering|Material|SetScalarParameterValue "/Game/Materials/MaterialLocationParameter.MaterialLocationParameter" "Actor X SP" (* (- (/ _x_2 _x) 0.5) -1.0) :!class /Script/Engine.KismetMaterialLibrary)
  (Rendering|Material|SetScalarParameterValue "/Game/Materials/MaterialLocationParameter.MaterialLocationParameter" "Actor Y SP" (* (- (/ _y_2 _y) 0.5) -1.0) :!class /Script/Engine.KismetMaterialLibrary))

(fn GroundOffset
  (bind _returnvalue (Transformation|GetActorLocation))
  (bind _returnvalue_2 (Transformation|GetActorLocation))
  (bind _returnvalue_3 (Transformation|GetActorLocation))
  (bind _returnvalue_4 (Transformation|GetActorLocation))
  (bind _angle (Variables|Default|GetAngle))
  (bind (_outhit _returnvalue_5) (Collision|LineTraceByChannel (+ _returnvalue "0, 0,200.000000") (- _returnvalue "0, 0,200.000000") "TraceTypeQuery1" false 0 "ForOneFrame" true "(R=0.000000,G=0.115952,B=1.000000,A=1.000000)"))
  (if _returnvalue_5
    (Transformation|AddActorWorldOffset (Math|Vector|MakeVector 0.0 0.0 (- (.Z (Math|Vector|BreakVector (.Location (Collision|BreakHitResult _outhit)))) (.Z (Math|Vector|BreakVector (Transformation|GetActorLocation))))))
    ;[1 1 1] Normalen til flaten under
    (Rendering|Debug|DrawDebugLine _returnvalue_3 (+ (* (.Normal (Collision|BreakHitResult _outhit)) 2e+02) _returnvalue_3) "(R=1.000000,G=0.000000,B=0.950916,A=1.000000)" 0.0 3.0)
    ;[1 1 1] Opp vektoren
    (Rendering|Debug|DrawDebugLine _returnvalue_4 (+ (* (Math|Vector|VectorUp) 2e+02) _returnvalue_4) "(R=0.070988,G=1.000000,B=0.000000,A=1.000000)" 0.0 3.0)
    ;[1 1 1] Roterte vektoren
    (Rendering|Debug|DrawDebugLine _returnvalue_2 (+ _returnvalue_2 (* (Math|Vector|Normalize (+ (* (.Normal (Collision|BreakHitResult _outhit)) (Math|Trig|Cos(Degrees) _angle)) (* (Math|Vector|CrossProduct (.Normal (Collision|BreakHitResult _outhit)) (Math|Vector|CrossProduct (Math|Vector|VectorUp) (.Normal (Collision|BreakHitResult _outhit)))) (Math|Trig|Sin(Degrees) _angle)))) 2e+02)) "(R=1.000000,G=0.078098,B=0.000000,A=1.000000)" 0.0 3.0)))